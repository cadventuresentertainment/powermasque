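; BP_Death_Plane is a box trigger that damages the player on contact.
; When the first player's pawn begins overlapping the box, a loop sends it TakeDamageMessage once per point of Damage.
; Each pass also plays one of three randomly chosen 2D sounds.
; The construction script sizes the box from the Extent variable.
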(event OnComponentBeginOverlap(Box)
  (params (OverlappedComponent :type Primitive%20Component%20Object%20Reference) (OtherActor :type Actor%20Object%20Reference) (OtherComp :type Primitive%20Component%20Object%20Reference) (OtherBodyIndex :type Integer) (bFromSweep :type Boolean) (SweepResult :type Hit%20Result%20Structure%20%28by%20ref%29))
  (bind _returnvalue (Game|Player|GetPlayerPawn 0))
  (if (== OtherActor _returnvalue)
    (for _index (range 1 (Variables|Properties|GetDamage))
      (Class|BPIPlayer|TakeDamage(Message) _returnvalue)
      (Audio|PlaySound2D (Utilities|Select :Index (Math|Random|RandomIntegerinRange 0 2) :Option%200 "/Game/Sounds/FX/S_Aah.S_Aah" :Option%201 "/Game/Sounds/FX/S_Auugghh.S_Auugghh" :Option%202 "/Game/Sounds/FX/S_Brazil.S_Brazil") 1.0 1.0 0.0 0 0))))

(fn ConstructionScript
  (Components|Box|SetBoxExtent (Variables|Default|GetBox) (Variables|Properties|GetExtent) true))